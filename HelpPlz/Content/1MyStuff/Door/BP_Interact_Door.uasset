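; BP_Interact_Door is an interactable door Blueprint that swings open and closed when a player interacts with it.
; The InteractwithObject event checks and flips IsDoorClosed, playing a Timeline forward to open or reversing it to close.
; The Timeline alpha drives a Lerp that sets the DoorMesh relative yaw between closed and a quarter turn open.
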(event `self.InteractWithObject`
  (if (`self.Is Door Closed`)
    (set `self.Is Door Closed` false)
    (bind (_direction _alpha) (`Timeline|Timeline` :!label _label)
      (:`Update`
        (`SceneComponent.K2_SetRelativeRotation` (`self.DoorMesh`) (`KismetMathLibrary.MakeRotator` 0.0 0.0 (`KismetMathLibrary.Lerp` 0.0 90.0 _alpha)) false false)))
    (else
      (set `self.Is Door Closed` true)
      (goto _label :!via `Reverse`))))

(fn `UserConstructionScript`
  (`parent.UserConstructionScript`))