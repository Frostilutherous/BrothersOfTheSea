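; BP_Master_Item is an item pickup actor that feeds into the AC_Inventory component of actors overlapping its InteractColl.
; On overlap it checks the component for BPI_InventoryInterface, then either auto-adds itself and is destroyed, or registers as the pickup candidate and shows the interaction prompt.
; Leaving deregisters it and hides the prompt once no overlapping items remain.
; Construction optionally enables mesh physics and collision, while the rotating-movement branch does nothing.
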(event `self.InteractColl.OnComponentBeginOverlap`
  (params (OverlappedComponent :type "PrimitiveComponent Object Reference") (OtherActor :type "Actor Object Reference") (OtherComp :type "PrimitiveComponent Object Reference") (OtherBodyIndex :type Integer) (bFromSweep :type Boolean) (SweepResult :type "HitResult Structure (by ref)"))
  (bind _returnvalue (`self.GetComponentByClass` OtherActor "/Game/1MyStuff/Inventory/AC_Inventory.AC_Inventory_C"))
  (if (`KismetSystemLibrary.DoesImplementInterface` _returnvalue "/Game/1MyStuff/Inventory/BPI_InventoryInterface.BPI_InventoryInterface_C")
    (if (`/Game/1MyStuff/Inventory/AC_Inventory.AutoPickup` _returnvalue)
      (`/Game/1MyStuff/Inventory/AC_Inventory.F_AddItemToInventory` _returnvalue self)
      (`self.K2_DestroyActor`)
      (else
        (`KismetArrayLibrary.Array_Add` (`/Game/1MyStuff/Inventory/AC_Inventory.OverlappingItems` _returnvalue) self)
        (set `/Game/1MyStuff/Inventory/AC_Inventory.ItemToPickup` self _returnvalue)
        (`/Game/1MyStuff/Inventory/AC_Inventory.SetInteractionVisibility` _returnvalue true)))))

(event `self.InteractColl.OnComponentEndOverlap`
  (params (OverlappedComponent :type "PrimitiveComponent Object Reference") (OtherActor :type "Actor Object Reference") (OtherComp :type "PrimitiveComponent Object Reference") (OtherBodyIndex :type Integer))
  (bind _returnvalue (`self.GetComponentByClass` OtherActor "/Game/1MyStuff/Inventory/AC_Inventory.AC_Inventory_C"))
  (bind _overlappingitems (`/Game/1MyStuff/Inventory/AC_Inventory.OverlappingItems` _returnvalue))
  (`/Engine/EditorBlueprintResources/StandardMacros.IsValid` OtherActor
    (:`Is Valid`
      (if (`KismetSystemLibrary.DoesImplementInterface` _returnvalue "/Game/1MyStuff/Inventory/BPI_InventoryInterface.BPI_InventoryInterface_C")
        (`KismetArrayLibrary.Array_RemoveItem` _overlappingitems self)
        (if (not (> (`KismetArrayLibrary.Array_Length` _overlappingitems) 0))
          (`/Game/1MyStuff/Inventory/AC_Inventory.SetInteractionVisibility` _returnvalue false))))))

(fn `UserConstructionScript`
  (if (`self.UsePhysics`)
    (`PrimitiveComponent.SetSimulatePhysics` (`self.StaticMesh`) true)
    (`PrimitiveComponent.SetCollisionEnabled` (`self.StaticMesh`) "QueryAndPhysics")
    (elif (`self.UseRotatingMovement`)
      _)))